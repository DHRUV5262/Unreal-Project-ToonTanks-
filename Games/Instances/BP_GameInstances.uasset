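; Game Instance that handles PlayFab accounts, matchmaking and dedicated-server (GSDK) hooks.
; Init sets a hardcoded title ID and secret key, registers GSDK delegates, mostly stubs except quit on shutdown, and signals readiness.
; Username login and registration store the entity token and open the main menu; email login is unwired.
; Matchmaking creates a DoOnce-guarded ticket with fixed region latency, polls until matched, then runs an open command using the server's IP and port.
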(event Custom|RegistrationSuccess
  (params (result :type Client%20Register%20Play%20Fab%20User%20Result%20Structure) (customData :type Object%20Object%20Reference))
  (bind (_entitytoken _playfabid) (Utilities|Struct|BreakClientRegisterPlayFabUserResult result))
  (Variables|Default|SetEntity%20Token_0 _entitytoken)
  (Variables|Default|SetPlay%20Fab%20Id _playfabid))

(event Custom|On_LoginWithUername
  (params (result :type Client%20Login%20Result%20Structure) (customData :type Object%20Object%20Reference))
  (bind (_entitytoken _playfabid) (Utilities|Struct|BreakClientLoginResult result))
  (Variables|Default|SetEntity%20Token_0 _entitytoken)
  (Variables|Default|SetPlay%20Fab%20Id _playfabid))

(event Custom|GSDKMaintenance
  (params (MaintenanceTime :type Date%20Time%20Structure%20%28by%20ref%29)))

(event Custom|GetMatchSuccess
  (params (result :type Multiplayer%20Get%20Match%20Result%20Structure) (customData :type Object%20Object%20Reference))
  (bind _serverdetails (Utilities|Struct|BreakMultiplayerGetMatchResult result))
  (Development|PrintString "getting into match")
  (bind _returnvalue (Class|PlayFabJsonObject|GetObjectArrayField _serverdetails "Ports"))
  (Development|PrintString (Utilities|String|Append "open " (Class|PlayFabJsonValue|AsString (Class|PlayFabJsonObject|GetField _serverdetails "IPV4Address")) ":" (Utilities|String|ToString(Float) (Class|PlayFabJsonObject|GetNumberField (Utilities|Array|Get(acopy) _returnvalue) "Num"))))
  (Development|ExecuteConsoleCommand (Utilities|String|Append "open " (Class|PlayFabJsonValue|AsString (Class|PlayFabJsonObject|GetField _serverdetails "IPV4Address")) ":" (Utilities|String|ToString(Float) (Class|PlayFabJsonObject|GetNumberField (Utilities|Array|Get(acopy) _returnvalue) "Num"))) 0))

(event Custom|ServerActiveDelegate)

(event Custom|ReadyForPlayer)

(event Custom|GetMatch
  (|GetMatch (Utilities|Struct|MakeMultiplayerGetMatchRequest 0 false (Variables|Default|GetMatch%20Id) "Test1") (delegate Custom|GetMatchSuccess) (EventDispatchers|CreateEvent :!event Custom|On_Failure_of_PlayFab)))

(event Custom|On_LoginwithEmail
  (params (result :type Client%20Login%20Result%20Structure) (customData :type Object%20Object%20Reference))
  (bind (_entitytoken _inforesultpayload _lastlogintime _newlycreated _playfabid) (Utilities|Struct|BreakClientLoginResult result))
  (Variables|Default|SetEntity%20Token_0 _entitytoken)
  (Variables|Default|SetPlay%20Fab%20Id _playfabid))

(event Custom|On_Failure_of_PlayFab
  (params (error :type Play%20Fab%20Error%20Structure) (customData :type Object%20Object%20Reference))
  (bind (_haserror _errorcode _errorname _errormessage _errordetails) (Utilities|Struct|BreakPlayFabError error))
  (Development|PrintString _errorname)
  (Development|PrintString _errordetails))

(event Custom|GSDKSutDownDelegate
  (Game|QuitGame 0 "Quit" false))

(event Custom|ResetMatchMaking
  (bind _returnvalue (Class|PlayFabJsonObject|ConstructJsonObject))
  (Utilities|FlowControl|DoOnce false) ; enters at Reset
)

(event Custom|MatchMakingSuccess
  (params (result :type Multiplayer%20Create%20Matchmaking%20Ticket%20Result%20Structure) (customData :type Object%20Object%20Reference))
  (Variables|Default|SetTicket%20Id (.TicketId (Utilities|Struct|BreakMultiplayerCreateMatchmakingTicketResult result)))
  (bind _returnvalue (Utilities|Time|SetTimerbyEvent (delegate Custom|Match%20Making%20Finder) 5.0 true))
  (Variables|Default|SetMatch%20Finder%20Timer%20Handle _returnvalue))

(event Custom|Match%20Making%20Finder
  (CallFunction|MatchFinder))

(event Custom|Match%20Finder
  (|GetMatchmakingTicket (Utilities|Struct|MakeMultiplayerGetMatchmakingTicketRequest 0 false "Test1" (Variables|Default|GetTicket%20Id)) (delegate Custom|FindMatch) (EventDispatchers|CreateEvent :!event Custom|On_Failure_of_PlayFab)))

(event Custom|FindMatch
  (params (result :type Multiplayer%20Get%20Matchmaking%20Ticket%20Result%20Structure) (customData :type Object%20Object%20Reference))
  (bind (_cancellationreasonstring _changenumber _created _creator _giveupafterseconds _matchid _members _memberstomatchwith _queuename _status) (Utilities|Struct|BreakMultiplayerGetMatchmakingTicketResult result))
  (Variables|Default|SetMatch%20Id _matchid)
  (Variables|Default|SetStatus _status)
  (if (Utilities|Enum|Equal(Enum) _status "Matched")
    (Utilities|Time|ClearandInvalidateTimerbyHandle (Variables|Default|GetMatch%20Finder%20Timer%20Handle))
    (Development|PrintString "Matched")
    (CallFunction|GetMatch)
    (else
      (Development|PrintString "failed"))))

(event EventInit
  (Class|PlayFabUtilities|SetPlayFabSettings "9BE50" "3NCNXAAB9DIXUYNSZPQ6I4RA6T3FIOO1M1W47ZOIJSRA8BTH8E")
  (Class|GSDKUtils|RegisterGSDKShutdownDelegate (delegate Custom|GSDKSutDownDelegate))
  (Class|GSDKUtils|RegisterGSDKHealthCheckDelegate (EventDispatchers|CreateEvent :!event BPGameInstancesAutoGenFunc))
  (Class|GSDKUtils|RegisterGSDKMaintenanceDelegate (delegate Custom|GSDKMaintenance))
  (Class|GSDKUtils|RegisterGSDKServerActiveDelegate (delegate Custom|ServerActiveDelegate))
  (Class|GSDKUtils|RegisterGSDKReadyforPlayers (delegate Custom|ReadyForPlayer))
  (Class|GSDKUtils|ReadyforPlayers))

(event EventRegister
  (params (username :type String) (emailid :type String) (password :type String))
  (bind _successful (|RegisterPlayFabUser (Utilities|Struct|MakeClientRegisterPlayFabUserRequest username emailid password username) (delegate Custom|RegistrationSuccess) (EventDispatchers|CreateEvent :!event Custom|On_Failure_of_PlayFab))
    (:OnPlayFabResponse
      (if _successful
        (Game|OpenLevel(byObjectReference) "/Game/MainMenu/MainMenu.MainMenu")))))

(event EventLogin
  (params (Uername/Email :type String) (password :type String))
  (bind _successful (|LoginwithPlayFab (Utilities|Struct|MakeClientLoginWithPlayFabRequest password Uername/Email) (delegate Custom|On_LoginWithUername) (EventDispatchers|CreateEvent :!event Custom|On_Failure_of_PlayFab))
    (:OnPlayFabResponse
      (if _successful
        (Game|OpenLevel(byObjectReference) "/Game/MainMenu/MainMenu.MainMenu")))))

(event EventStartMatchMaking
  (bind _returnvalue (Class|PlayFabJsonObject|ConstructJsonObject))
  (Utilities|FlowControl|DoOnce false
    (:Completed
      (Variables|Default|SetLatency%20Item _returnvalue)
      (Variables|Default|Setlatencies _returnvalue)
      (Variables|Default|SetAttributes _returnvalue)
      (Variables|Default|SetDataObject _returnvalue)
      (bind _output_get (Variables|Default|SetCreator%20Settings _returnvalue))
      (Class|PlayFabJsonObject|SetStringField (Variables|Default|GetLatency%20Item) "Region" "EastUs")
      (Class|PlayFabJsonObject|SetStringField (Variables|Default|GetLatency%20Item) "latency" "150")
      (Class|PlayFabJsonObject|SetArrayField (Variables|Default|Getlatencies) "Latencies" (Utilities|Array|MakeArray (Class|PlayFabJsonValue|ConstructJsonValueObject (Variables|Default|GetLatency%20Item))))
      (Class|PlayFabJsonObject|SetObjectField (Variables|Default|GetDataObject) "DataObject" (Variables|Default|Getlatencies))
      (Class|PlayFabJsonObject|SetObjectField (Variables|Default|GetCreator%20Settings) "Entity" (Class|PlayFabJsonObject|GetObjectField (Variables|Default|GetEntity%20Token_0) "Entity"))
      (Class|PlayFabJsonObject|SetObjectField (Variables|Default|GetCreator%20Settings) "Attributes" (Variables|Default|GetDataObject))
      (|MatchmakingTicket (Utilities|Struct|MakeMultiplayerCreateMatchmakingTicketRequest _output_get 90 "Test1") (delegate Custom|MatchMakingSuccess) (EventDispatchers|CreateEvent :!event Custom|On_Failure_of_PlayFab)))))

(fn BPGameInstancesAutoGenFunc1
  (return true))

(fn BPGameInstancesAutoGenFunc
  (return true))

(fn GetMatchMaking)

(fn GetMatchMakingStatus
  (return (Variables|Default|GetStatus)))